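; Utility actor that previews lighting and rendering feature sets for different target hardware tiers.
; Switch functions store their settings and run console commands for GI, reflections, AO, shadows, Lumen ray tracing and anti-aliasing.
; The construction script reapplies the stored settings, except anti-aliasing, whenever it runs.
; Five preset functions, from last-gen console to hardware ray tracing, call every switch and print the targeted tier.
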(event EventBeginPlay)

(event Collision|EventActorBeginOverlap
  (params (OtherActor :type Actor%20Object%20Reference)))

(event EventTick
  (params (DeltaSeconds :type Float%20%28single-precision%29)))

(fn ConstructionScript
  (Helpers|SwitchGI (Variables|LightingFeatures|GlobalIllumination|GetSelectDynamicGI_Method))
  (Helpers|SwitchReflections (Variables|LightingFeatures|Reflection|GetSelectReflectionMethod))
  (Helpers|SwitchAO (Variables|LightingFeatures|AmbientOcclusion|GetEnableSSAO) (Variables|LightingFeatures|AmbientOcclusion|GetEnableDFAO))
  (Helpers|SwitchShadows (Variables|LightingFeatures|Shadow|GetEnableContactShadow) (Variables|LightingFeatures|Shadow|GetEnableCapsuleDirectShadow) (Variables|LightingFeatures|Shadow|GetEnableCapsuleIndirectShadow) (Variables|LightingFeatures|Shadow|GetEnableDistanceFieldShadow) (Variables|LightingFeatures|Shadow|GetEnablePerObjectShadow) (Variables|LightingFeatures|Shadow|GetEnableVirtualShadowMap))
  (Helpers|SwitchLumenMode (Variables|LightingFeatures|LumenMode|GetEnableLumenHWRT) (Variables|LightingFeatures|LumenMode|GetEnableLumenHWRT_HitLighting)))

(fn SwitchGI
  (params (SelectDynamicGI_Method :type ELightingMethodsSwitchGI%20Enum :default "NewEnumerator2"))
  (Utilities|FlowControl|Sequence
    (:then_0
      (Variables|LightingFeatures|GlobalIllumination|SetSelectDynamicGI_Method SelectDynamicGI_Method))
    (:then_1
      (Development|ExecuteConsoleCommand (Utilities|Select :Index (Variables|LightingFeatures|GlobalIllumination|GetSelectDynamicGI_Method) :NewEnumerator0 "r.DynamicGlobalIlluminationMethod 0" :NewEnumerator1 "r.DynamicGlobalIlluminationMethod 2" :NewEnumerator2 "r.DynamicGlobalIlluminationMethod 1") 0) ; Switch GI
    )))

(fn SwitchReflections
  (params (SelectReflectionMethod :type ELightingMethodsSwitchReflection%20Enum :default "NewEnumerator2"))
  (Utilities|FlowControl|Sequence
    (:then_0
      (Variables|LightingFeatures|Reflection|SetSelectReflectionMethod SelectReflectionMethod))
    (:then_1
      (Development|ExecuteConsoleCommand (Utilities|Select :Index (Variables|LightingFeatures|Reflection|GetSelectReflectionMethod) :NewEnumerator0 "r.ReflectionMethod 0" :NewEnumerator1 "r.ReflectionMethod 2" :NewEnumerator2 "r.ReflectionMethod 1") 0) ; Switch reflection method
    )))

(fn SwitchAO
  (params (EnableSSAO :type Boolean) (EnableDFAO :type Boolean))
  (Utilities|FlowControl|Sequence
    (:then_0
      (Variables|LightingFeatures|AmbientOcclusion|SetEnableSSAO EnableSSAO)
      (Variables|LightingFeatures|AmbientOcclusion|SetEnableDFAO EnableDFAO))
    (:then_1
      (Development|ExecuteConsoleCommand (select (Variables|LightingFeatures|AmbientOcclusion|GetEnableSSAO) "r.AmbientOcclusionRadiusScale 1" "r.AmbientOcclusionRadiusScale 0") 0) ; SSAO
      (Development|ExecuteConsoleCommand (select (Variables|LightingFeatures|AmbientOcclusion|GetEnableDFAO) "r.DistanceFieldAO 1" "r.DistanceFieldAO 0") 0) ; DFAO
    )))

(fn SwitchShadows
  (params (EnableContactShadow :type Boolean) (EnableCapsuleDirectShadow :type Boolean) (EnableCapsuleIndirectShadow :type Boolean) (EnableDistanceFieldShadow :type Boolean) (EnablePerObjectShadow :type Boolean) (EnableVirtualShadowMap :type Boolean))
  (Utilities|FlowControl|Sequence
    (:then_0
      (Variables|LightingFeatures|Shadow|SetEnableContactShadow EnableContactShadow)
      (Variables|LightingFeatures|Shadow|SetEnableCapsuleDirectShadow EnableCapsuleDirectShadow)
      (Variables|LightingFeatures|Shadow|SetEnableCapsuleIndirectShadow EnableCapsuleIndirectShadow)
      (Variables|LightingFeatures|Shadow|SetEnableDistanceFieldShadow EnableDistanceFieldShadow)
      (Variables|LightingFeatures|Shadow|SetEnablePerObjectShadow EnablePerObjectShadow)
      (Variables|LightingFeatures|Shadow|SetEnableVirtualShadowMap EnableVirtualShadowMap))
    (:then_1
      (Development|ExecuteConsoleCommand (select (Variables|LightingFeatures|Shadow|GetEnableContactShadow) "r.ContactShadows 1" "r.ContactShadows 0") 0) ; Contact
      (Development|ExecuteConsoleCommand (select (Variables|LightingFeatures|Shadow|GetEnableCapsuleDirectShadow) "r.CapsuleDirectShadows 1" "r.CapsuleDirectShadows 0") 0) ; Capsule
      (Development|ExecuteConsoleCommand (select (Variables|LightingFeatures|Shadow|GetEnableCapsuleIndirectShadow) "r.CapsuleIndirectShadows 1" "r.CapsuleIndirectShadows 0") 0) ; Capsule
      (Development|ExecuteConsoleCommand (select (Variables|LightingFeatures|Shadow|GetEnableDistanceFieldShadow) "r.DistanceFieldShadowing 1" "r.DistanceFieldShadowing 0") 0) ; DF shadow
      (Development|ExecuteConsoleCommand (select (Variables|LightingFeatures|Shadow|GetEnableVirtualShadowMap) "r.Shadow.Virtual.Enable 1" "r.Shadow.Virtual.Enable 0") 0) ; VSM
      (Development|ExecuteConsoleCommand (select (Variables|LightingFeatures|Shadow|GetEnablePerObjectShadow) "r.Shadow.PerObject 1" "r.Shadow.PerObject 0") 0) ; Per object
    )))

(fn SwitchLumenMode
  (params (EnableLumenHWRT :type Boolean) (EnableLumenHWRT_HitLighting :type Boolean))
  (Utilities|FlowControl|Sequence
    (:then_0
      (Variables|LightingFeatures|LumenMode|SetEnableLumenHWRT EnableLumenHWRT)
      (Variables|LightingFeatures|LumenMode|SetEnableLumenHWRT_HitLighting EnableLumenHWRT_HitLighting))
    (:then_1
      (Development|ExecuteConsoleCommand (select (Variables|LightingFeatures|LumenMode|GetEnableLumenHWRT) "r.Lumen.HardwareRayTracing 1" "r.Lumen.HardwareRayTracing 0") 0) ; Switch between SRT and HRT
      (Development|ExecuteConsoleCommand (select (Variables|LightingFeatures|LumenMode|GetEnableLumenHWRT_HitLighting) "r.Lumen.HardwareRayTracing.LightingMode 2" "r.Lumen.HardwareRayTracing.LightingMode 0") 0) ; HRT Hit
    )))

(fn 0-LowestPreset
  (Helpers|SwitchGI "NewEnumerator0")
  (Helpers|SwitchReflections "NewEnumerator0")
  (Helpers|SwitchAO true false)
  (Helpers|SwitchShadows true true true false true false)
  (Helpers|SwitchLumenMode false false)
  (Helpers|SwitchAAMethod "NewEnumerator0")
  (Development|PrintString (Utilities|String|Append "Message: 
" "Lowest Preset - PS4/XBOX ONE Target Hardware.") true true "(R=0.000000,G=1.000000,B=0.589859,A=1.000000)" 5.0))

(fn 1-MediumLowPreset
  (Helpers|SwitchGI "NewEnumerator0")
  (Helpers|SwitchReflections "NewEnumerator1")
  (Helpers|SwitchAO true false)
  (Helpers|SwitchShadows true true true true true false)
  (Helpers|SwitchLumenMode false false)
  (Helpers|SwitchAAMethod "NewEnumerator1")
  (Development|PrintString (Utilities|String|Append "Message: 
" "Medium - Low Preset - AMD POLARIS (RX580 and above) / NVIDIA TURING (GTX1660 and above) Target Hardware.") true true "(R=0.000000,G=1.000000,B=0.589859,A=1.000000)" 5.0))

(fn 2-MediumPreset
  (Helpers|SwitchGI "NewEnumerator1")
  (Helpers|SwitchReflections "NewEnumerator1")
  (Helpers|SwitchAO true true)
  (Helpers|SwitchShadows true true true true true false)
  (Helpers|SwitchLumenMode false false)
  (Helpers|SwitchAAMethod "NewEnumerator1")
  (Development|PrintString (Utilities|String|Append "Message: 
" "Medium Preset - AMD RDNA 2 (RX6600 and above) / NVIDIA TURING (RTX2060 and above) Target Hardware.") true true "(R=0.000000,G=1.000000,B=0.589859,A=1.000000)" 5.0))

(fn 3-HighPreset
  (Helpers|SwitchGI "NewEnumerator2")
  (Helpers|SwitchReflections "NewEnumerator2")
  (Helpers|SwitchAO true true)
  (Helpers|SwitchShadows true true true true true true)
  (Helpers|SwitchLumenMode false false)
  (Helpers|SwitchAAMethod "NewEnumerator3")
  (Development|PrintString (Utilities|String|Append "Message: 
" "High Preset - AMD RDNA 2 (RX6800 and above) / NVIDIA AMPERE (RTX3070 and above) Target Hardware.") true true "(R=0.000000,G=1.000000,B=0.589859,A=1.000000)" 5.0))

(fn 4-ExtremePreset
  (Helpers|SwitchGI "NewEnumerator2")
  (Helpers|SwitchReflections "NewEnumerator2")
  (Helpers|SwitchAO false true)
  (Helpers|SwitchShadows true true true true true true)
  (Helpers|SwitchLumenMode true true)
  (Helpers|SwitchAAMethod "NewEnumerator3")
  (Development|PrintString (Utilities|String|Append "Message: 
" "Extreme Preset - Hardware Ray-Tracing.") true true "(R=0.000000,G=1.000000,B=0.589859,A=1.000000)" 5.0))

(fn SwitchAAMethod
  (params (AAMethod :type ELightingMethodsSwitchAA%20Enum :default "NewEnumerator0"))
  (Utilities|FlowControl|Sequence
    (:then_0
      (Variables|LightingFeatures|AAMethod|SetAAMethod AAMethod))
    (:then_1
      (Development|ExecuteConsoleCommand (Utilities|Select :Index (Variables|LightingFeatures|AAMethod|GetAAMethod) :NewEnumerator0 "r.AntiAliasingMethod 1" :NewEnumerator1 "r.AntiAliasingMethod 2" :NewEnumerator3 "r.AntiAliasingMethod 4") 0) ; Switch reflection method
    )))